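; Spike hazard actor that deals fixed damage to a MyCharacter overlapping its Spikes component.
; It reduces the character's Health directly, then either prints a survival warning or, below zero, prints a death message, destroys the spike actor itself and reloads the current level.
; Actor begin overlap and Spikes end overlap both set Trigger true, toggle WarnPlayer visibility and invoke CallTrue.
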(event OnComponentBeginOverlap(Spikes)
  (params (OtherActor :type Actor%20Object%20Reference) (OtherComp :type Primitive%20Component%20Object%20Reference) (OtherBodyIndex :type Integer) (bFromSweep :type Boolean) (SweepResult :type Hit%20Result%20Structure%20%28by%20ref%29))
  ;[1 1 1] Spikes
  (bind _asmy_character (Utilities|Casting|CastToMyCharacter OtherActor))
  (bind _output_get (Variables|/Game/Blueprints/MyCharacter.MyCharacter_C|SetHealth _asmy_character (- (Variables|/Game/Blueprints/MyCharacter.MyCharacter_C|GetHealth _asmy_character) 25.0)))
  (Math|Float|CompareFloat _output_get 0.0
    (:>
      (Development|PrintString "Still Alive! Be Careful!" true true "(R=1.000000,G=0.934895,B=0.000000,A=1.000000)" 3.0))
    (:<
      (Development|PrintString "You're killed!" true true "(R=1.000000,G=0.000000,B=0.016322,A=1.000000)" 3.0)
      (Actor|DestroyActor)
      (bind _returnvalue (Game|GetCurrentLevelName true))
      (Game|OpenLevel(byName) (Utilities|String|StringToName _returnvalue)))))

(event OnComponentEndOverlap(Spikes)
  (params (OtherActor :type Actor%20Object%20Reference) (OtherComp :type Primitive%20Component%20Object%20Reference) (OtherBodyIndex :type Integer))
  (Variables|Default|SetTrigger true)
  (if (Variables|Default|GetTrigger)
    (Rendering|ToggleVisibility (Variables|Default|GetWarn%20player) false)
    (Default|CallTrue)))

(event EventBeginPlay)

(event EventTick
  (params (DeltaSeconds :type Float%20%28single-precision%29)))

(event EventActorBeginOverlap
  (params (OtherActor :type Actor%20Object%20Reference))
  ;[1 1 1] Show Text When Actor Overlaps
  (Variables|Default|SetTrigger true)
  (if (Variables|Default|GetTrigger)
    (Rendering|ToggleVisibility (Variables|Default|GetWarn%20player) false)
    (Default|CallTrue)))

(fn ConstructionScript)