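; AgroCheck is a ticking Behavior Tree service that detects aggro targets around the AI's controlled pawn.
; Each tick sphere-traces for nearby objects, then line-traces on the Camera channel to test line of sight, ignoring one actor class.
; Visible hits write TargetToFollow and TargetLocation to the Blackboard, while blocked hits clear only TargetToFollow.
; The loop never breaks, so the last hit processed decides the target.
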(event EventTick
  (params (OwnerActor :type Actor%20Object%20Reference) (DeltaSeconds :type Float%20%28single-precision%29))
  (bind _returnvalue (Pawn|GetControlledPawn))
  (bind _returnvalue_2 (Transformation|GetActorLocation _returnvalue))
  ;[1 1 1] Is AI_CON_Ref set?
  (if (!= 0 0)
    _
    (else
      (Utilities|Casting|CastTo OwnerActor)
      (Variables|Default|SetAI_CON_Ref 0)))
  (bind _outactors (Actor|GetAllActorsOfClass 0))
  (Variables|Default|SetMyLocation _returnvalue_2)
  (bind _outhits (Collision|MultiSphereTraceForObjects _returnvalue_2 (+ _returnvalue_2 "0, 0,15.000000") 1.5e+03 (Variables|Default|GetDesiredObjectTypes) false _outactors "None"))
  (bind _array_element (Utilities|Array|ForEachLoopwithBreak _outhits)
    (:LoopBody
      (bind _outhit (Collision|LineTraceByChannel (Variables|Default|GetMyLocation) (Transformation|GetActorLocation (.HitActor (Collision|BreakHitResult _array_element))) "TraceTypeQuery2" false _outactors "None"))
      (if (== (.HitActor (Collision|BreakHitResult _outhit)) (.HitActor (Collision|BreakHitResult _array_element)))
        (Class|BTFunctionLibrary|SetBlackboardValueasObject (Variables|Default|GetTargetToFollow) (.HitActor (Collision|BreakHitResult _outhit)))
        (AI|BehaviorTree|SetBlackboardValueasVector (Variables|Default|GetTargetLocation) (Transformation|GetActorLocation (.HitActor (Collision|BreakHitResult _outhit))))
        (else
          (Class|BTFunctionLibrary|SetBlackboardValueasObject (Variables|Default|GetTargetToFollow)))))))