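; Fire is a short-lived item actor that raises the player character's mood while they stand near it.
; After a short delay it activates the Fire component and caches the player, then deactivates and destroys itself 20 seconds later.
; Trigger overlaps toggle an in-range flag, which a looping timer checks to add small clamped increments to the character's MoodValue.
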(event OnComponentBeginOverlap(Trigger)
  (params (OtherActor :type Actor%20Object%20Reference) (OtherComp :type Primitive%20Component%20Object%20Reference) (OtherBodyIndex :type Integer) (bFromSweep :type Boolean) (SweepResult :type Hit%20Result%20Structure%20%28by%20ref%29))
  ;[1 1 1] Trigger
  (Utilities|Casting|CastToMyCharacter OtherActor)
  (Variables|Default|SetIsInRange true))

(event OnComponentEndOverlap(Trigger)
  (params (OtherActor :type Actor%20Object%20Reference) (OtherComp :type Primitive%20Component%20Object%20Reference) (OtherBodyIndex :type Integer))
  ;[1 1 1] Trigger
  (Utilities|Casting|CastToMyCharacter OtherActor)
  (Variables|Default|SetIsInRange false))

(event Custom|IncreaseMood
  (bind _mycharacter (Variables|Default|GetMyCharacter))
  ;[1 1 1] Increase Mood Event (Loops Every 1.5 seconds)
  (if (Variables|Default|GetIsInRange)
    (Variables|/Game/Blueprints/MyCharacter.MyCharacter_C|SetMoodValue _mycharacter (Math|Float|Clamp(Float) (+ (Variables|/Game/Blueprints/MyCharacter.MyCharacter_C|GetMoodValue _mycharacter) 0.05)))))

(event EventBeginPlay
  (bind _fire (Variables|Default|GetFire))
  ;[1 1 1] Event Begin Play
  (Utilities|FlowControl|Delay 2.0)
  (Components|Activation|Activate _fire false)
  (bind _asmy_character (Utilities|Casting|CastToMyCharacter (Game|GetPlayerCharacter 0)))
  (Variables|Default|SetMyCharacter _asmy_character)
  (Utilities|Time|SetTimerbyFunctionName self "IncreaseMood" 1.5 true)
  (Utilities|FlowControl|Delay 2e+01)
  (Components|Activation|Deactivate _fire)
  (Actor|DestroyActor))

(fn ConstructionScript)